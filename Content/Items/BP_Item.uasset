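; BP_Item is a world pickup actor that adds its ItemObject to the top-down character's inventory on sphere overlap.
; BeginPlay fills a missing ItemObject via GetDefaultItemObject, empty here, caches the player and hides the decal.
; Clicking the mesh shows the decal and stores its location.
; Successful adds destroy the actor, but PickupItem and last-picked-up value (GoldValue times grid area) update even when adding fails.
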(event OnComponentBeginOverlap(Sphere)
  (params (OverlappedComponent :type Primitive%20Component%20Object%20Reference) (OtherActor :type Actor%20Object%20Reference) (OtherComp :type Primitive%20Component%20Object%20Reference) (OtherBodyIndex :type Integer) (bFromSweep :type Boolean) (SweepResult :type Hit%20Result%20Structure%20%28by%20ref%29))
  (bind _item_object (Variables|Private|GetItem%20Object))
  (bind _dimensions (Default|GetDimensions _item_object))
  (bind _asbp_top_down_character (Utilities|Casting|CastToBP_TopDownCharacter OtherActor))
  (Utilities|FlowControl|Sequence
    (:then_0
      (bind _added (Default|TryAddItem (Variables|/Game/TopDown/Blueprints/BP_TopDownCharacter.BP_TopDownCharacter_C|GetBP_InventoryComponent _asbp_top_down_character) (Variables|Private|GetItem%20Object)))
      (if _added
        (Actor|DestroyActor)))
    (:then_1
      (Default|PickupItem (Variables|Default|GetCharacterRef))
      (Variables|/Game/Inventory/BP_InventoryComponent.BP_InventoryComponent_C|SetLastPickedUpItemValue (Variables|/Game/TopDown/Blueprints/BP_TopDownCharacter.BP_TopDownCharacter_C|GetBP_InventoryComponent (Variables|Default|GetCharacterRef)) (* (Variables|/Game/Items/BP_ItemObject.BP_ItemObject_C|GetGoldValue _item_object) (* (.x _dimensions) (.y _dimensions)))))))

(event OnClicked(StaticMesh)
  (params (TouchedComponent :type Primitive%20Component%20Object%20Reference) (ButtonPressed :type Key%20Structure :default "None"))
  (CallFunction|ItemClicked)
  (Variables|Default|SetTargetedItemLocation (Transformation|GetWorldLocation TouchedComponent)))

(event Custom|ItemClicked
  (Development|SetHiddeninGame (Variables|Default|GetDecal) false false))

(event EventBeginPlay
  (Utilities|FlowControl|Sequence
    (:then_0
      (if (not (Utilities|IsValid (Variables|Private|GetItem%20Object)))
        (bind _itemobject (CallFunction|GetDefaultItemObject))
        (Variables|Private|SetItem%20Object _itemobject)))
    (:then_1
      (bind _asbp_top_down_character (Utilities|Casting|CastToBP_TopDownCharacter (Game|GetPlayerCharacter 0)))
      (Variables|Default|SetCharacterRef _asbp_top_down_character))
    (:then_2
      (Development|SetHiddeninGame (Variables|Default|GetDecal) true false))))

(fn ConstructionScript)

(fn GetDefaultItemObject
  (return 0))